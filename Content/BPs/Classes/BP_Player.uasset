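; BP_Player is the player character Blueprint, handling contact damage and death through a HealthComponent.
; A capsule hit on another BaseCharacter applies Damage to that character's HealthComponent, then triggers its health bar update event.
; The player's own UpdateHealthBar event destroys the actor when current health reaches zero or below; it fetches the health percentage but never uses it.
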(event `self.ReceiveBeginPlay`)

(event `self.UpdateHealthBar`
  (`HealthComponent.GetHealthPercentage` (`self.HealthComponent`))
  (bind _returnvalue (`HealthComponent.GetCurrentHealth` (`self.HealthComponent`)))
  (if (<= _returnvalue 0)
    (`self.K2_DestroyActor`)))

(event `self.CapsuleComponent.OnComponentHit`
  (params (HitComponent :type "PrimitiveComponent Object Reference") (OtherActor :type "Actor Object Reference") (OtherComp :type "PrimitiveComponent Object Reference") (NormalImpulse :type "Vector Structure") (Hit :type "HitResult Structure (by ref)"))
  (bind _asbase_character (cast `BaseCharacter` OtherActor))
  (`HealthComponent.TakeDamage` (`BaseCharacter.HealthComponent` _asbase_character) (`self.Damage`))
  (`self.CallUpdateHealthBarEvent` _asbase_character))

(fn `UserConstructionScript`)