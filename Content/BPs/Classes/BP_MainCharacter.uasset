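; BP_MainCharacter is the main character Blueprint, which keeps a health bar widget in sync with its health.
; On BeginPlay it binds to the HealthComponent's OnHealthUpdate dispatcher and calls an update event.
; The bound handler casts the WidgetHealthBar component's widget to WBP_HealthBar and sets its progress bar from the component's health percentage, so updates are event-driven without Tick.
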(event `self.ReceiveBeginPlay`
  (add `HealthComponent.OnHealthUpdate` (`self.HealthComponent`) (delegate `OnHealthUpdate_Event`))
  (`self.OnHealthUpdate_Event`))

(event `OnHealthUpdate_Event`
  (bind _aswbp_health_bar (cast `/Game/BPs/Widgets/WBP_HealthBar` (`WidgetComponent.GetWidget` (`self.WidgetHealthBar`))))
  (bind _returnvalue (`HealthComponent.GetHealthPercentage` (`self.HealthComponent`)))
  (`ProgressBar.SetPercent` (`/Game/BPs/Widgets/WBP_HealthBar.HealthBar` _aswbp_health_bar) _returnvalue))

(fn `UserConstructionScript`)