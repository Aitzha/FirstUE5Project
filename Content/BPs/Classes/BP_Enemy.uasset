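; BP_Enemy is an enemy actor with a health bar that deals contact damage to characters.
; A capsule hit on a BaseCharacter applies Damage to that character's HealthComponent and triggers its health bar update.
; UpdateHealthBar copies the enemy's HealthComponent percentage into its WBP_HealthBar widget and destroys the enemy at zero health, so the death check runs only when that event is called.
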(event `self.ReceiveBeginPlay`)

(event `self.UpdateHealthBar`
  (bind _aswbp_health_bar (cast `/Game/BPs/Widgets/WBP_HealthBar` (`WidgetComponent.GetWidget` (`self.HealthBarWidget`))))
  (bind _returnvalue (`HealthComponent.GetHealthPercentage` (`self.HealthComponent`)))
  (`ProgressBar.SetPercent` (`/Game/BPs/Widgets/WBP_HealthBar.HealthBar` _aswbp_health_bar) _returnvalue)
  (bind _returnvalue_2 (`HealthComponent.GetCurrentHealth` (`self.HealthComponent`)))
  (if (<= _returnvalue_2 0)
    (`self.K2_DestroyActor`)))

(event `self.CapsuleComponent.OnComponentHit`
  (params (HitComponent :type "PrimitiveComponent Object Reference") (OtherActor :type "Actor Object Reference") (OtherComp :type "PrimitiveComponent Object Reference") (NormalImpulse :type "Vector Structure") (Hit :type "HitResult Structure (by ref)"))
  (bind _asbase_character (cast `BaseCharacter` OtherActor))
  (`HealthComponent.TakeDamage` (`BaseCharacter.HealthComponent` _asbase_character) (`self.Damage`))
  (`self.CallUpdateHealthBarEvent` _asbase_character))

(fn `UserConstructionScript`)